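; Player-controlled rolling ball pawn that moves by physics and keeps a running points score.
; Two movement axes apply torque to the Sphere, scaled by Speed as an acceleration change, and AddPoints adds to Points.
; Two camera functions set spring arm length and rotation, one in world space, the other relative, which also feeds arm length into roll.
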(event `InputAxis|ForwardBackMovement`
  (params (AxisValue :type "Float (single-precision)"))
  ;[1 1 1] uni video, + speed from yt, ball now moves
  (`PrimitiveComponent.AddTorqueInRadians` (`self.Sphere`) (`KismetMathLibrary.MakeVector` 0.0 (* AxisValue (`self.Speed`))) "None" true))

(event `InputAxis|LeftRIghtMovement`
  (params (AxisValue :type "Float (single-precision)"))
  ;[1 1 1] uni video, + speed from yt, ball now moves
  (`PrimitiveComponent.AddTorqueInRadians` (`self.Sphere`) (`KismetMathLibrary.MakeVector` (* AxisValue (`self.Speed`))) "None" true))

(event `AddPoints`
  (params (PointValue :type Integer))
  ;[1 1 1] point system from a yt video
  (set `self.Points` (+ PointValue (`self.Points`))))

(fn `change camera view`
  (params (`camera position` :type "Float (double-precision)") (`camera rotation y` :type "Float (double-precision)") (`camera rotation z` :type "Float (double-precision)"))
  (bind _springarm (`self.SpringArm`))
  (set `SpringArmComponent.TargetArmLength` `camera position` _springarm)
  (`SceneComponent.K2_SetWorldRotation` _springarm (`KismetMathLibrary.MakeRotator` 0.0 `camera rotation y` `camera rotation z`) false false))

(fn `change camera view 02`
  (params (`camera distance` :type "Float (double-precision)") (`camera rotation y` :type "Float (double-precision)") (`camera rotation Z` :type "Float (double-precision)"))
  (bind _springarm (`self.SpringArm`))
  (bind _output_get (set `SpringArmComponent.TargetArmLength` `camera distance` _springarm))
  (`SceneComponent.K2_SetRelativeRotation` _springarm (`KismetMathLibrary.MakeRotator` _output_get `camera rotation y` `camera rotation Z`) false false))

(fn `UserConstructionScript`)